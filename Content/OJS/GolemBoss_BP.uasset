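; Golem boss that roams random reachable points and breaks off to approach a sensed, nearby player and play an attack montage.
; Tick updates the chase, health bar and death check, while a looping timer calls LoseHealth, which is not defined here.
; A sphere overlap shows or removes the boss bar, and mesh contact damages the player, ending in a paused game-over screen.
; The AnyDamage handler is empty, with its old logic left disconnected.
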(event `self.ReceiveTick`
  (params (DeltaSeconds :type "Float (single-precision)"))
  ;[1 1 1] Tick Event
  (`self.UpdatePawnChase`)
  (`self.updateHeathBar`)
  (`self.CheckHealth`))

(event `self.ReceiveBeginPlay`
  (`KismetSystemLibrary.K2_SetTimer` null "LoseHealth" 0.5 true)
  ;[1 1 1] begin Play
  (`self.Roam`))

(event `Roam`
  ;[1 1 1] Roam
  (if (`self.isDead`)
    _
    (elif (`self.isRoaming`)
      _
      (elif (not (`self.isAttacking`))
        (set `self.isRoaming` true)
        (`|AIMoveTo` self (`NavigationSystemV1.K2_GetRandomReachablePointInRadius` (`self.K2_GetActorLocation`) 2500.0 null null) null 250.0
          (:`OnSuccess`
            _)
          (:`OnFail`
            _))
        (`KismetSystemLibrary.Delay` 3.0)
        (set `self.isRoaming` false)
        (`self.Roam`)))))

(event `self.PawnSensing.OnSeePawn`
  (params (Pawn :type "Pawn Object Reference"))
  ;[1 1 1] event - see pawn
  (set `self.chasingPawn` Pawn))

(event `UpdatePawnChase`
  ;[1 1 1] update Pawn Chase
  (`/Engine/EditorBlueprintResources/StandardMacros.IsValid` (`self.chasingPawn`)
    (:`Is Valid`
      (if (< (`KismetMathLibrary.Vector_Distance` (`self.K2_GetActorLocation` (`self.chasingPawn`)) (`self.K2_GetActorLocation`)) 2500.0)
        (if (`self.isDead`)
          _
          (elif (not (`self.isAttacking`))
            (set `self.isAttacking` true)
            (`Controller.StopMovement` (`AIBlueprintHelperLibrary.GetAIController` self))
            (`|AIMoveTo` self (0.0 0.0 0.0) (`self.chasingPawn`) 500.0
              (:`OnSuccess`
                (bind _returnvalue (`self.PlayAnimMontage` "/Game/OJS/boosAttack_Montage.boosAttack_Montage"))
                (`KismetSystemLibrary.Delay` _returnvalue))
              (:`OnFail`
                _))
            (set `self.isAttacking` false)
            (`self.Roam`)))))
    (:`Is Not Valid`
      (`self.Roam`))))

(event `self.Sphere.OnComponentBeginOverlap`
  (params (OverlappedComponent :type "PrimitiveComponent Object Reference") (OtherActor :type "Actor Object Reference") (OtherComp :type "PrimitiveComponent Object Reference") (OtherBodyIndex :type Integer) (bFromSweep :type Boolean) (SweepResult :type "HitResult Structure (by ref)"))
  (cast `/Game/ThirdPerson/Blueprints/BP_ThirdPersonCharacter` OtherActor)
  (bind _returnvalue (`|CreateWidget` "/Game/BOSS/BossBar/BossHealthBar.BossHealthBar_C"))
  (`UserWidget.AddToViewport` _returnvalue 0)
  (bind _asboss_health_bar (cast `/Game/BOSS/BossBar/BossHealthBar` _returnvalue)))

(event `self.Sphere.OnComponentEndOverlap`
  (params (OverlappedComponent :type "PrimitiveComponent Object Reference") (OtherActor :type "Actor Object Reference") (OtherComp :type "PrimitiveComponent Object Reference") (OtherBodyIndex :type Integer))
  (cast `/Game/ThirdPerson/Blueprints/BP_ThirdPersonCharacter` OtherActor)
  (`Widget.RemoveFromParent` (stale `self.Sphere.OnComponentBeginOverlap` _returnvalue)))

(event `updateHeathBar`
  ;[1 1 1] update Healthbar
  (bind _asboss_health_bar (cast `/Game/BOSS/BossBar/BossHealthBar` (stale `self.Sphere.OnComponentBeginOverlap` _asboss_health_bar)))
  (`ProgressBar.SetPercent` (`/Game/BOSS/BossBar/BossHealthBar.ProgressBar_Boss` _asboss_health_bar) (/ (`self.Health`) (`self.MaxHeath`))))

(event `CheckHealth`
  ;[1 1 1] Check Health  Death
  (if (<= (`self.Health`) 0)
    (set `self.isDead` true)
    (`Controller.StopMovement` (`AIBlueprintHelperLibrary.GetAIController` self))
    (`KismetSystemLibrary.Delay` 1.0)
    (`self.K2_DestroyActor`)))

(event `self.Mesh.OnComponentBeginOverlap`
  (params (OverlappedComponent :type "PrimitiveComponent Object Reference") (OtherActor :type "Actor Object Reference") (OtherComp :type "PrimitiveComponent Object Reference") (OtherBodyIndex :type Integer) (bFromSweep :type Boolean) (SweepResult :type "HitResult Structure (by ref)"))
  (bind _returnvalue (`GameplayStatics.GetPlayerController` 0))
  ;[1 1 1] Player 데미지 받
  (bind _asbp_third_person_character (cast `/Game/ThirdPerson/Blueprints/BP_ThirdPersonCharacter` OtherActor))
  (`GameplayStatics.SpawnEmitterAtLocation` "/Game/InfinityBladeEffects/Effects/FX_Monsters/FX_Monster_SpiderBoss/Fire/P_Spider_Lava_Roar.P_Spider_Lava_Roar" (`self.K2_GetActorLocation`) (struct) (3.0 3.0 3.0))
  (bind _resulthp (`/Game/ThirdPerson/Blueprints/BP_ThirdPersonCharacter.Damage` _asbp_third_person_character 0.2))
  (if (<= _resulthp 0.0)
    (`self.K2_DestroyActor` _asbp_third_person_character)
    ;[1 1 1] GameOver 화면에 뜨게
    (bind _returnvalue_2 (`|CreateWidget` "/Game/ThirdPerson/Blueprints/UI/UMG_GameOver.UMG_GameOver_C"))
    (`UserWidget.AddToViewport` _returnvalue_2 0)
    (set `PlayerController.bShowMouseCursor` true _returnvalue)
    (`WidgetBlueprintLibrary.SetInputMode_UIOnlyEx` _returnvalue null)
    (`GameplayStatics.SetGamePaused` true)))

(event `self.Mesh.OnComponentEndOverlap`
  (params (OverlappedComponent :type "PrimitiveComponent Object Reference") (OtherActor :type "Actor Object Reference") (OtherComp :type "PrimitiveComponent Object Reference") (OtherBodyIndex :type Integer))
  ;[1 1 1] collision box 나갔을 시 어택중지해라
)

(event `self.ReceiveAnyDamage`
  (params (Damage :type "Float (single-precision)") (DamageType :type "DamageType Object Reference") (InstigatedBy :type "Controller Object Reference") (DamageCauser :type "Actor Object Reference"))
  ;[1 1 1] Line Trace로 데미지 받는방법/////프로젝트에 사용안함
)

(fn `UserConstructionScript`)