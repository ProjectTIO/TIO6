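; Golem enemy that roams random navmesh points, chases a pawn it has sensed, and drops loot when killed.
; Tick drives the chase within range: AIMoveTo, attack montage, then roaming resumes; mesh overlap damages the player.
; A bullet or fireball hit destroys it instantly and spawns one of four random loot classes at a reachable point nearby.
; Health and timed-attack logic are disconnected.
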(event `drop loot`
  (bind _returnvalue (`self.K2_GetActorLocation`))
  (bind _outhit (`KismetSystemLibrary.LineTraceSingle` _returnvalue (- _returnvalue (0.0 0.0 200.0)) "TraceTypeQuery1" false (`|MakeArray` (`GameplayStatics.GetPlayerCharacter` 0) :!type "Actor Object Reference")))
  (`|SpawnActorFromClass` (select `int` (`KismetMathLibrary.RandomInteger` 4) :`0` "/Game/OJS/item/LootDrop.LootDrop_C" :`1` "/Game/OJS/item/LootDrop2.LootDrop2_C" :`2` "/Game/OJS/item/LootDrop3.LootDrop3_C" :`3` "/Game/OJS/item/LootDrop4.LootDrop4_C" :!type "Actor Class Reference") (`KismetMathLibrary.MakeTransform` (`NavigationSystemV1.K2_GetRandomReachablePointInRadius` (`.Location` (`GameplayStatics.BreakHitResult` _outhit)) 250.0 null null) (`KismetMathLibrary.MakeRotator` 0.0 0.0 (`KismetMathLibrary.RandomFloatInRange` 0.0 360.0))) "Undefined" "MultiplyWithRoot" null null))

(event `self.ReceiveHit`
  (params (MyComp :type "PrimitiveComponent Object Reference") (Other :type "Actor Object Reference") (OtherComp :type "PrimitiveComponent Object Reference") (bSelfMoved :type Boolean) (HitLocation :type "Vector Structure") (HitNormal :type "Vector Structure") (NormalImpulse :type "Vector Structure") (Hit :type "HitResult Structure (by ref)"))
  (`|ExecutionSequence`
    (:`then_0`
      (bind _asbp_bullet (cast `/Game/ThirdPerson/Blueprints/BP_Bullet` Other)))
    (:`then_1`
      (bind _asbp_fire_ball (cast `/Game/ThirdPerson/Blueprints/BP_FireBall` Other))))
  (`self.K2_DestroyActor` _asbp_bullet)
  (`self.K2_DestroyActor` _asbp_fire_ball)
  (`self.K2_DestroyActor` self)
  (`self.drop loot`))

(event `self.ReceiveTick`
  (params (DeltaSeconds :type "Float (single-precision)"))
  ;[1 1 1] Tick Event
  (`self.UpdatePawnChase`))

(event `self.ReceiveBeginPlay`
  ;[1 1 1] begin Play
  (`self.Roam`))

(event `Roam`
  ;[1 1 1] Roam
  (if (`self.isDead`)
    _
    (elif (`self.isRoaming`)
      _
      (elif (not (`self.isAttacking`))
        (set `self.isRoaming` true)
        (`|AIMoveTo` self (`NavigationSystemV1.K2_GetRandomReachablePointInRadius` (`self.K2_GetActorLocation`) 1500.0 null null) null 200.0
          (:`OnSuccess`
            _)
          (:`OnFail`
            _))
        (`KismetSystemLibrary.Delay` 3.0)
        (set `self.isRoaming` false)
        (`self.Roam`)))))

(event `self.PawnSensing.OnSeePawn`
  (params (Pawn :type "Pawn Object Reference"))
  ;[1 1 1] event - see pawn
  (set `self.chasingPawn` Pawn))

(event `UpdatePawnChase`
  ;[1 1 1] update Pawn Chase
  (`/Engine/EditorBlueprintResources/StandardMacros.IsValid` (`self.chasingPawn`)
    (:`Is Valid`
      (if (< (`KismetMathLibrary.Vector_Distance` (`self.K2_GetActorLocation` (`self.chasingPawn`)) (`self.K2_GetActorLocation`)) 2500.0)
        (if (`self.isDead`)
          _
          (elif (not (`self.isAttacking`))
            (set `self.isAttacking` true)
            (`Controller.StopMovement` (`AIBlueprintHelperLibrary.GetAIController` self))
            (`|AIMoveTo` self (0.0 0.0 0.0) (`self.chasingPawn`) 300.0
              (:`OnSuccess`
                (bind _returnvalue (`self.PlayAnimMontage` "/Game/OJS/item/MobAttack_Montage.MobAttack_Montage"))
                (`KismetSystemLibrary.Delay` _returnvalue))
              (:`OnFail`
                _))
            (set `self.isAttacking` false)
            (`self.Roam`)))))
    (:`Is Not Valid`
      (`self.Roam`))))

(event `self.Mesh.OnComponentBeginOverlap`
  (params (OverlappedComponent :type "PrimitiveComponent Object Reference") (OtherActor :type "Actor Object Reference") (OtherComp :type "PrimitiveComponent Object Reference") (OtherBodyIndex :type Integer) (bFromSweep :type Boolean) (SweepResult :type "HitResult Structure (by ref)"))
  (bind _asbp_third_person_character (cast `/Game/ThirdPerson/Blueprints/BP_ThirdPersonCharacter` OtherActor))
  (`/Game/ThirdPerson/Blueprints/BP_ThirdPersonCharacter.Damage` _asbp_third_person_character 0.1))

(event `Attack`
  (bind _asbp_third_person_character (cast `/Game/ThirdPerson/Blueprints/BP_ThirdPersonCharacter` (`GameplayStatics.GetPlayerCharacter` 0)))
  (`/Game/ThirdPerson/Blueprints/BP_ThirdPersonCharacter.Damage` _asbp_third_person_character 10.0))

(event `self.Box.OnComponentEndOverlap`
  (params (OverlappedComponent :type "PrimitiveComponent Object Reference") (OtherActor :type "Actor Object Reference") (OtherComp :type "PrimitiveComponent Object Reference") (OtherBodyIndex :type Integer))
  ;[1 1 1] collision box 나갔을 시 어택중지해라
  (cast `/Game/ThirdPerson/Blueprints/BP_ThirdPersonCharacter` OtherActor)
  ;;[1 1 1] 타이머중지
  (`KismetSystemLibrary.K2_ClearAndInvalidateTimerHandle` (`self.AttackTimer`)))

(event `self.ReceiveAnyDamage`
  (params (Damage :type "Float (single-precision)") (DamageType :type "DamageType Object Reference") (InstigatedBy :type "Controller Object Reference") (DamageCauser :type "Actor Object Reference"))
  ;[1 1 1] Line Trace로 데미지 받는방법/////프로젝트에 사용안함
)

(fn `NewFunction`)

(fn `UserConstructionScript`)