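; BOMB_BP is a bomb actor whose Explode event plays a large explosion and breaks Chaos destructible objects around it.
; Explode spawns the particle effect at the actor, then applies an external cluster strain field with radial falloff, centered on and sized by the Sphere component.
; Sphere overlap casts for BP_Bullet but triggers nothing, as the Explode call in this graph is disconnected.
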(event `Explode`
  (bind _sphere (`self.Sphere`))
  (`GameplayStatics.SpawnEmitterAtLocation` "/Game/InfinityBladeEffects/P_Explosion.P_Explosion" (`self.K2_GetActorLocation`) (struct) (7.7 7.7 7.7))
  (`FieldSystemComponent.ApplyPhysicsField` (`self.FieldSystemComponent`) true "Field_ExternalClusterStrain" null (`RadialFalloff.SetRadialFalloff` (`self.RadialFalloff`) 500000.0 0.0 2.0 0.0 (`SphereComponent.GetScaledSphereRadius` _sphere) (`SceneComponent.K2_GetComponentLocation` _sphere) "Field_FallOff_None")))

(event `self.Sphere.OnComponentBeginOverlap`
  (params (OverlappedComponent :type "PrimitiveComponent Object Reference") (OtherActor :type "Actor Object Reference") (OtherComp :type "PrimitiveComponent Object Reference") (OtherBodyIndex :type Integer) (bFromSweep :type Boolean) (SweepResult :type "HitResult Structure (by ref)"))
  (cast `/Game/ThirdPerson/Blueprints/BP_Bullet` OtherActor))

(fn `UserConstructionScript`)