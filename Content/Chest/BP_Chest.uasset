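; BP_Chest is an interactable treasure chest whose opening ends the game with a win sequence.
; Its trigger overlap shows and hides a widget component while something is in range.
; InteractwithChest plays a sound and the open animation, then uses chained delays to show a found-item widget, clear all widgets, play a win sound and display the game-end screen with mouse cursor, UI-only input and the game paused.
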(event `/Game/Chest/intractInterface.interactWithChest`
  (bind _returnvalue (`GameplayStatics.GetPlayerController` 0))
  (`GameplayStatics.PlaySound2D` "/Game/Chest/dorm-door-opening-6038__online-audio-converter_com_.dorm-door-opening-6038__online-audio-converter_com_" 1.0 1.0 0.0 null null)
  (`SkeletalMeshComponent.PlayAnimation` (`self.chest`) "/Game/Models/treasure-chest/source/Chest_Anim_Armature_A_Open.Chest_Anim_Armature_A_Open" false)
  (`KismetSystemLibrary.Delay` 3.0)
  (bind _returnvalue_2 (`|CreateWidget` "/Game/Chest/UMG_findITEM.UMG_findITEM_C"))
  (`UserWidget.AddToViewport` _returnvalue_2 0)
  (`KismetSystemLibrary.Delay` 6.0)
  (`WidgetLayoutLibrary.RemoveAllWidgets`)
  (`KismetSystemLibrary.Delay` 3.0)
  (`GameplayStatics.PlaySound2D` "/Game/ThirdPerson/Blueprints/Sounds/piglevelwin2mp3-14800.piglevelwin2mp3-14800" 1.0 1.0 0.0 null null)
  ;[1 1 1] GameOver 화면에 뜨게
  (bind _returnvalue_3 (`|CreateWidget` "/Game/Chest/UMG_GameEnd.UMG_GameEnd_C"))
  (`UserWidget.AddToViewport` _returnvalue_3 0)
  (set `PlayerController.bShowMouseCursor` true _returnvalue)
  (`WidgetBlueprintLibrary.SetInputMode_UIOnlyEx` _returnvalue null)
  (`GameplayStatics.SetGamePaused` true))

(event `self.Trigger.OnComponentBeginOverlap`
  (params (OverlappedComponent :type "PrimitiveComponent Object Reference") (OtherActor :type "Actor Object Reference") (OtherComp :type "PrimitiveComponent Object Reference") (OtherBodyIndex :type Integer) (bFromSweep :type Boolean) (SweepResult :type "HitResult Structure (by ref)"))
  (`SceneComponent.SetVisibility` (`self.Widget`) true false))

(event `self.Trigger.OnComponentEndOverlap`
  (params (OverlappedComponent :type "PrimitiveComponent Object Reference") (OtherActor :type "Actor Object Reference") (OtherComp :type "PrimitiveComponent Object Reference") (OtherBodyIndex :type Integer))
  (`SceneComponent.SetVisibility` (`self.Widget`) false false))

(fn `UserConstructionScript`)