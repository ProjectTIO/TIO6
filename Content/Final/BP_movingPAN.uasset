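; BP_movingPAN is a moving "pan" actor driven by an InterpToMovement component.
; Its MOVINGpan function adds two absolute control points, the world origin and the MoveToPos variable, to define the path.
; Nothing in these graphs calls that function.
; Relative-position versions of the same setup sit unexecuted in the event graph and construction script.
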(fn `MOVINGpan`
  (`InterpToMovementComponent.AddControlPointPosition` (`self.InterpToMovement`) (0.0 0.0 0.0) false)
  (`InterpToMovementComponent.AddControlPointPosition` (`self.InterpToMovement`) (`self.moveToPos`) false))

(fn `UserConstructionScript`)