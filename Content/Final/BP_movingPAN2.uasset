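; BP_movingPAN2 is an actor that moves continuously along its forward vector once its Hit33 event is triggered; nothing in this graph calls that event.
; Hit33 re-arms itself through a near-zero timer and offsets the location by Speed times world delta seconds, without sweeping, instead of using Tick.
; The construction script and MovingPan2 function are empty, leaving only unconnected InterpToMovement control-point nodes toward MovetoPOS.
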(event `Hit33`
  ;[1 1 1] 살아가면서 앞방향으로 계속 이동하고 싶다.
  (`KismetSystemLibrary.K2_SetTimerDelegate` (delegate `Hit33`) 0.0001)
  (`self.K2_SetActorLocation` (+ (`self.K2_GetActorLocation`) (* (`self.GetActorForwardVector`) (`self.speed`) (`GameplayStatics.GetWorldDeltaSeconds`)))))

(fn `MovingPan2`)

(fn `UserConstructionScript`)